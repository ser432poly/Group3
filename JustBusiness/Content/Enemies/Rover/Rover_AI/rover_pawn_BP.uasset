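; Rover enemy pawn that periodically fires shots from its gun socket.
; Each Tick counts down a shot timer; at zero it spawns a Rover_shot at the RoverBody socket, resets the timer to a random value and plays a positional sound with randomized volume and pitch.
; The timer counts frames rather than seconds, so fire rate depends on framerate.
; A drift direction is exposed through simple get and set functions.
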(event `self.ReceiveBeginPlay`)

(event `self.ReceiveActorBeginOverlap`
  (params (OtherActor :type "Actor Object Reference")))

(event `self.ReceiveTick`
  (params (DeltaSeconds :type "Float (single-precision)"))
  (if (<= (`self.ShotTimer`) 0)
    (`|SpawnActorFromClass` "/Game/rover_shot.rover_shot_C" (`SceneComponent.GetSocketTransform` (`self.rover_body`) "GunSocket" "RTS_World") "Undefined" "OverrideRootScale")
    (set `self.ShotTimer` (`KismetMathLibrary.RandomIntegerInRange` 25 75))
    (`GameplayStatics.PlaySoundAtLocation` "/Game/SoundEffects/StarWars_RogueSquadron/BANK_00_INSTR_0082_SND_0000.BANK_00_INSTR_0082_SND_0000" (`self.K2_GetActorLocation` self) (struct) (`KismetMathLibrary.RandomFloatInRange` 0.7 1.0) (`KismetMathLibrary.RandomFloatInRange` 1.0 1.3) 0.0 "/Game/SoundEffects/Modifiers/ShootSound.ShootSound")
    (else
      (`/Engine/EditorBlueprintResources/StandardMacros.DecrementInt` (`self.ShotTimer`)))))

(fn `GetDriftDir`
  (returns (DriftDir :type "Vector Structure"))
  (return (`self.DriftDir`)))

(fn `SetDriftDir`
  (params (inDriftDir :type "Vector Structure"))
  (set `self.DriftDir` inDriftDir)
  (return))

(fn `UserConstructionScript`)