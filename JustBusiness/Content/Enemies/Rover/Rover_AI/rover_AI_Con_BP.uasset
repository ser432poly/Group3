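; AI controller for the Rover enemy that starts its behavior tree.
; On BeginPlay it sets up the Rover blackboard, zeroes the target score zone center and stores the controlled pawn as MyPawn.
; It then runs RoverBT, leaving further logic to the tree; Tick is unused.
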(event `self.ReceiveBeginPlay`
  (`self.UseBlackboard` "/Game/Enemies/Rover/Rover_AI/RoverBlackboard.RoverBlackboard")
  (`BlackboardComponent.SetValueAsVector` (`AIBlueprintHelperLibrary.GetBlackboard` self) (`self.TargetScoreZoneCenter`) (0.0 0.0 0.0))
  (`BlackboardComponent.SetValueAsObject` (`AIBlueprintHelperLibrary.GetBlackboard` self) (`self.my_pawn`) (`self.K2_GetPawn`))
  (`self.RunBehaviorTree` "/Game/Enemies/Rover/Rover_AI/RoverBT.RoverBT"))

(event `self.ReceiveTick`
  (params (DeltaSeconds :type "Float (single-precision)")))

(fn `UserConstructionScript`)