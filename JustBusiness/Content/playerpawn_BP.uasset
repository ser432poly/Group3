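; Player ship pawn with health, twin-gun primary fire, engine audio pitch control and a pause menu hookup.
; Overlapping a KillZone-tagged actor applies heavy environmental damage; AnyDamage reduces Health and calls Death below zero, which spawns an explosion and destroys visual components, not the actor.
; FirePrimary spawns shots from both gun sockets with randomized sound, while point damage attaches a minor explosion to the ship.
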(event `self.ReceiveBeginPlay`)

(event `self.Sphere.OnComponentBeginOverlap`
  (params (OtherActor :type "Actor Object Reference") (OtherComp :type "PrimitiveComponent Object Reference") (OtherBodyIndex :type Integer) (bFromSweep :type Boolean) (SweepResult :type "HitResult Structure (by ref)"))
  (if (`self.ActorHasTag` OtherActor "KillZone")
    (`GameplayStatics.ApplyDamage` self 200.0 null null "/Engine/EngineDamageTypes/DmgTypeBP_Environmental.DmgTypeBP_Environmental_C")))

(event `self.ReceiveTick`
  (params (DeltaSeconds :type "Float (single-precision)")))

(event `self.ReceiveAnyDamage`
  (params (Damage :type "Float (single-precision)") (DamageType :type "DamageType Object Reference") (InstigatedBy :type "Controller Object Reference") (DamageCauser :type "Actor Object Reference"))
  (bind _returnvalue (- (`self.Health`) Damage))
  (if (< _returnvalue 0.0)
    (set `self.Health` 0.0)
    (`self.Death`)
    (else
      (set `self.Health` _returnvalue))))

(event `self.ReceivePointDamage`
  (params (Damage :type "Float (single-precision)") (DamageType :type "DamageType Object Reference") (HitLocation :type "Vector Structure") (HitNormal :type "Vector Structure") (HitComponent :type "PrimitiveComponent Object Reference") (BoneName :type Name) (ShotFromDirection :type "Vector Structure") (InstigatedBy :type "Controller Object Reference") (DamageCauser :type "Actor Object Reference"))
  (`GameplayStatics.SpawnEmitterAttached` "/Game/StarterContent/Particles/P_Explosion_Minor.P_Explosion_Minor" (`self.ship`)))

(event `InputAction|PauseMenu`
  (params (Key :type "Key Structure" :default "AnyKey"))
  (:`Pressed`
    (`GameplayStatics.SetGamePaused` null true)
    (bind _returnvalue (`|CreateWidget` "/Game/UI/InGameMenu.InGameMenu_C"))
    (`UserWidget.AddToViewport` _returnvalue 0)
    (set `PlayerController.bShowMouseCursor` true (`GameplayStatics.GetPlayerController` null))))

(fn `Death`
  (`GameplayStatics.SpawnEmitterAtLocation` null "/Game/StarterContent/Particles/P_Explosion.P_Explosion" (`self.K2_GetActorLocation` self))
  (`ActorComponent.K2_DestroyComponent` (`self.ship`))
  (`ActorComponent.K2_DestroyComponent` (`self.Cube`))
  (`ActorComponent.K2_DestroyComponent` (`self.d1`))
  (`ActorComponent.K2_DestroyComponent` (`self.d2`))
  (`ActorComponent.K2_DestroyComponent` (`self.d3`))
  (`ActorComponent.K2_DestroyComponent` (`self.d4`)))

(fn `FirePrimary`
  (`|SpawnActorFromClass` "/Game/shot.shot_C" (`SceneComponent.GetSocketTransform` (`self.ship`) "GunSocketR" "RTS_World") "Undefined" "OverrideRootScale" self)
  (`|SpawnActorFromClass` "/Game/shot.shot_C" (`SceneComponent.GetSocketTransform` (`self.ship`) "GunSocketL" "RTS_World") "Undefined" "OverrideRootScale" self)
  (`GameplayStatics.PlaySoundAtLocation` null "/Game/SoundEffects/StarWars_RogueSquadron/BANK_00_INSTR_0079_SND_0000.BANK_00_INSTR_0079_SND_0000" (`SceneComponent.K2_GetComponentLocation` (`self.Sphere`)) (struct) (`KismetMathLibrary.RandomFloatInRange` 0.7 1.0) (`KismetMathLibrary.RandomFloatInRange` 1.0 1.3)))

(fn `SetAudioPitch`
  (params (NewPitch :type "Float (double-precision)"))
  (`AudioComponent.SetPitchMultiplier` (`self.EngineSound`) NewPitch)
  (return))

(fn `UserConstructionScript`)