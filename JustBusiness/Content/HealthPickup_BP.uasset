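; Health pickup actor that heals the player pawn when overlapped.
; The first overlap by a playerpawn_BP sets a collected flag, calls Heal with HealAmount and spawns a particle effect at the pickup's location.
; Once collected, Tick shrinks the actor toward zero scale with a per-frame lerp and destroys it when it is nearly invisible.
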(event `self.ReceiveBeginPlay`)

(event `self.ReceiveActorBeginOverlap`
  (params (OtherActor :type "Actor Object Reference"))
  (if (not (`self.isCollected`))
    (bind _asplayerpawn_bp (cast `/Game/playerpawn_BP` OtherActor))
    (set `self.isCollected` true)
    (`/Game/playerpawn_BP.Heal` _asplayerpawn_bp (`self.HealAmount`))
    (`GameplayStatics.SpawnEmitterAtLocation` "/Game/P_health_particles.P_health_particles" (`self.K2_GetActorLocation` self))))

(event `self.ReceiveTick`
  (params (DeltaSeconds :type "Float (single-precision)"))
  (if (`self.isCollected`)
    (`self.SetActorScale3D` self (`KismetMathLibrary.VLerp` (`self.GetActorScale3D` self) (0.0 0.0 0.0) 0.1))
    (if (< (`KismetMathLibrary.VSize` (`self.GetActorScale3D` self)) 0.01)
      (`self.K2_DestroyActor`))))

(fn `UserConstructionScript`)